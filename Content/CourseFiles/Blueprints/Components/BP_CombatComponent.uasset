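; Combat component that holds its owner's combat state: main weapon, combat mode, blocking, shield-equipped flag, attack combo and dodge montages.
; Setting a new main weapon unequips and destroys the previous one, and ResetAttack clears the attack count and saved attack.
; Combat, blocking and shield setters broadcast event dispatchers, with blocking firing only on a change.
; SetShieldWeapon is an empty stub, and BeginPlay and Tick are unused.
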(event EventBeginPlay)

(event EventTick
  (params (DeltaSeconds :type Float%20%28single-precision%29)))

(fn SetMainWeapon
  (params (NewWeapon :type BP%20Base%20Weapon%20Object%20Reference))
  (Utilities|FlowControl|Sequence
    (:then_0
      (Utilities|IsValid (Variables|Default|GetMainWeapon)
        (:Is%20Valid
          ;[1 1 1] Need to check if weapon is valid/ equipped, then destroy if there already is a weapon
          (Default|OnUnequipped (Variables|Default|GetMainWeapon))
          (Actor|DestroyActor (Variables|Default|GetMainWeapon)))))
    (:then_1
      (Variables|Default|SetMainWeapon NewWeapon))))

(fn GetMainWeapon
  (return (Variables|Default|GetMainWeapon)))

(fn SetCombatEnabled
  (params (bEnableCombat :type Boolean))
  (bind _output_get (Variables|Default|SetbCombatEnabled? bEnableCombat))
  (Default|CallOnCombatToggled _output_get))

(fn IsCombatEnabled?
  (return (Variables|Default|GetbCombatEnabled?)))

(fn ResetAttack
  (Variables|Default|SetAttackCount 0)
  (Variables|Default|SetbIsAttackSaved false))

(fn GetDodgeMontages
  (return (Variables|Default|GetDodgeMontages)))

(fn SetBlockingState
  (params (bEnableBlocking :type Boolean))
  (if (!= bEnableBlocking (Variables|Default|GetbIsBlocking))
    (bind _output_get (Variables|Default|SetbIsBlocking bEnableBlocking))
    (Default|CallOnBlockingSet _output_get)))

(fn SetShieldWeapon
  (params (InShield :type BP%20Base%20Weapon%20Object%20Reference)))

(fn IsBlocking
  (return (Variables|Default|GetbIsBlocking)))

(fn IsShieldEquipped
  (return (Variables|Default|GetbIsShieldEquipped?)))

(fn SetShieldEquipped
  (params (Equipped :type Boolean))
  (bind _output_get (Variables|Default|SetbIsShieldEquipped? Equipped))
  (Default|CallOnShieldEquipped _output_get))