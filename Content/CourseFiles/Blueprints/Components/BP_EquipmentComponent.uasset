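; Equipment component that manages the items its owning actor has equipped, spawning them from a starting list on initialization.
; Equipping replaces any item of the same class, spawns the new actor at the owner and stores it in EquippedItems.
; Unequipping destroys the item and drops its pickup class at the owner, without removing the array entry.
; Gameplay-tag searches return an equipped item or trigger its action, using the first match.
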(event EventBeginPlay)

(event EventTick
  (params (DeltaSeconds :type Float%20%28single-precision%29)))

(fn InitializeEquipment
  (Utilities|FlowControl|Sequence
    (:then_0
      (for _array_element (Variables|Default|GetEquippedItems)
        (CallFunction|UnequipItem _array_element)))
    (:then_1
      (for _array_element_2 (Variables|Initalization|GetStartingEquipment)
        (if (Utilities|IsValidClass _array_element_2)
          (CallFunction|EquipItem _array_element_2)))
      (return))))

(fn PerformActionfromItem
  (params (Item%20Tag :type Gameplay%20Tag%20Structure))
  (for _array_element (Variables|Default|GetEquippedItems)
    (Utilities|IsValid _array_element
      (:Is%20Valid
        (bind _returnvalue (Default|HasMatchingGameplayTag _array_element Item%20Tag))
        (if _returnvalue
          (Default|PerformItemAction _array_element)
          (return)))))
  (return))

(fn GetEquippedItembyTag
  (params (ItemTag :type Gameplay%20Tag%20Structure))
  (for _array_element (Variables|Default|GetEquippedItems)
    (Utilities|IsValid _array_element
      (:Is%20Valid
        (bind _returnvalue (Default|HasMatchingGameplayTag _array_element ItemTag))
        (if _returnvalue
          (return _array_element)))))
  (return 0))

(fn EquipItem
  (params (InEquipment :type BP%20Base%20Equipable%20Class%20Reference))
  (bind _returnvalue (Components|GetOwner))
  (bind _aspawn (Utilities|Casting|CastToPawn _returnvalue))
  (if (Utilities|IsValidClass InEquipment)
    (Utilities|FlowControl|Sequence
      (:then_0
        (for _array_element (Variables|Default|GetEquippedItems)
          (if (== (Utilities|GetClass _array_element) InEquipment)
            (CallFunction|UnequipItem _array_element))))
      (:then_1
        (bind _returnvalue_2 (Game|SpawnActorfromClass InEquipment (Transformation|GetActorTransform _returnvalue) "Undefined" "MultiplyWithRoot" _aspawn _aspawn))
        (Default|OnEquipped _returnvalue_2)
        (Utilities|Array|AddUnique (Variables|Default|GetEquippedItems) _returnvalue_2)
        (return true)))
    (else
      (return false))))

(fn UnequipItem
  (params (EquipmentToUnequip :type BP%20Base%20Equipable%20Object%20Reference))
  (Utilities|IsValid EquipmentToUnequip
    (:Is%20Valid
      (Default|OnUnequipped EquipmentToUnequip)
      (CallFunction|SpawnEquipmentonGround (Variables|/Game/CourseFiles/Blueprints/Actors/BP_BaseEquipable.BP_BaseEquipable_C|GetPickUpItem EquipmentToUnequip))
      (Actor|DestroyActor EquipmentToUnequip))))

(fn UnequipAllItems
  (for _array_element (Variables|Default|GetEquippedItems)
    (CallFunction|UnequipItem _array_element)))

(fn SpawnEquipmentonGround
  (params (InEquipment :type BP%20Pickup%20Actor%20Class%20Reference))
  (bind _returnvalue (Components|GetOwner))
  (bind _aspawn (Utilities|Casting|CastToPawn _returnvalue))
  (if (Utilities|IsValidClass InEquipment)
    (Game|SpawnActorfromClass InEquipment (Transformation|GetActorTransform _returnvalue) "Undefined" "MultiplyWithRoot" _aspawn _aspawn)
    (return true)
    (else
      (return false))))