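; Collision component that detects hits along a mesh, sphere-tracing between its start and end sockets every tick while collision is active.
; Activating clears the already-hit list, so each actor registers only once per activation.
; Hits are filtered by ignored gameplay tags, already-hit actors and an editable ignore list, then broadcast through OnHit.
; The owner supplies the mesh and toggles collision through events.
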(event Custom|ActivateCollision
  (CallFunction|ClearHitActors)
  (Variables|Default|SetbIsCollisionEnabled? true))

(event Custom|DeactivateCollision
  (Variables|Default|SetbIsCollisionEnabled? false))

(event Custom|CollisionTrace
  (bind _collisionmeshcomponent (Variables|Default|GetCollisionMeshComponent))
  ;[1 1 1] Collision Trace
  (bind _outhits (Collision|MultiSphereTraceForObjects (Transformation|GetSocketLocation _collisionmeshcomponent (Variables|Initialization|GetStart%20Socket%20Name)) (Transformation|GetSocketLocation _collisionmeshcomponent (Variables|Initialization|GetEnd%20Socket%20Name)) (Variables|Initialization|GetTraceRadius) (Variables|Initialization|GetCollisionObject%20Types) false (Variables|Default|GetActors%20to%20Ignore) (Variables|Initialization|GetDraw%20Debug%20Type)))
  (for _array_element _outhits
    (bind _output_get (Variables|Default|SetLastHit _array_element))
    (if (CallFunction|CanHitActor? (.HitActor (Collision|BreakHitResult _output_get)))
      (bind _output_get_2 (Variables|Default|SetHit%20Actor (.HitActor (Collision|BreakHitResult _output_get))))
      (Utilities|Array|Add (Variables|Default|GetAlreadyHitActors) _output_get_2)
      (Default|CallOnHit (Variables|Default|GetLastHit)))))

(event Custom|ClearHitActors
  (Utilities|Array|Clear (Variables|Default|GetAlreadyHitActors)))

(event Custom|SetCollisionMesh
  (params (MeshComponent :type Primitive%20Component%20Object%20Reference))
  (Variables|Default|SetCollisionMeshComponent MeshComponent))

(event EventBeginPlay)

(event EventTick
  (params (DeltaSeconds :type Float%20%28single-precision%29))
  (if (Variables|Default|GetbIsCollisionEnabled?)
    (CallFunction|CollisionTrace)))

(fn GetAlreadyHitActors
  (return (Variables|Default|GetAlreadyHitActors)))

(fn IsCollisionEnabled?
  (return (Variables|Default|GetbIsCollisionEnabled?)))

(fn GetLastHit
  (return (Variables|Default|GetLastHit)))

(fn GetCollisionMesh
  (return (Variables|Default|GetCollisionMeshComponent)))

(fn AddActortoIgnore
  (params (InActor :type Actor%20Object%20Reference%20%28by%20ref%29))
  (Utilities|Array|AddUnique (Variables|Default|GetActors%20to%20Ignore) InActor))

(fn RemoveActortoIgnore
  (params (InActorToRemove :type Actor%20Object%20Reference%20%28by%20ref%29))
  (Utilities|Array|RemoveItem (Variables|Default|GetActors%20to%20Ignore) InActorToRemove))

(fn GetActorstoIgnore
  (return (Variables|Default|GetActors%20to%20Ignore)))

(fn CanHitActor?
  (params (InActor :type Actor%20Object%20Reference%20%28by%20ref%29))
  (bind _returnvalue (Class|GameplayTagBlueprintInterface|GetOwnedGameplayTags(Message) InActor))
  (return (Math|Boolean|ANDBoolean (not (GameplayTags|HasAnyTags _returnvalue (Variables|Default|GetGameplayTagsToIgnore) true)) (not (Utilities|Array|ContainsItem (Variables|Default|GetAlreadyHitActors) InActor)) (not (Utilities|Array|ContainsItem (Variables|Default|GetActorsToIgnore) (Utilities|GetClass InActor))))))