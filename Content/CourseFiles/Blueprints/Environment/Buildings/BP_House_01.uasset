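; BP_House_01 is a house building Blueprint with villager mobs and a health bar.
; On BeginPlay it sets its gameplay tag and registers its villager mob array before running the parent's BeginPlay.
; It then creates a WB_BuildingHealthBar widget bound to its BuildingStatsComponent, assigns it to HealthBar and hides the building health.
; The construction script only calls the parent; overlap and tick events are disabled.
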(event EventBeginPlay
  (CallFunction|SetGameplayTag (Variables|Default|GetTag))
  (CallFunction|AddVillagerMobArray (Variables|Default|GetVillagerMobs))
  (|CallParentFunction)
  (bind _returnvalue (UserInterface|CreateWidget "/Game/CourseFiles/UI/WB_BuildingHealthBar.WB_BuildingHealthBar_C" (Game|GetPlayerController 0) (Variables|Default|GetBuildingStatsComponent)))
  (UserInterface|SetWidget (Variables|Default|GetHealthBar) _returnvalue)
  (CallFunction|SetBuildingHealthInvisible))

(event Collision|EventActorBeginOverlap
  (params (OtherActor :type Actor%20Object%20Reference))
  (|CallParentFunction OtherActor) ; This node is disabled and will not be called.\nDrag off pins to build functionality.
)

(event EventTick
  (params (DeltaSeconds :type Float%20%28single-precision%29))
  (|CallParentFunction DeltaSeconds) ; This node is disabled and will not be called.\nDrag off pins to build functionality.
)

(fn ConstructionScript
  (|CallParentFunction))