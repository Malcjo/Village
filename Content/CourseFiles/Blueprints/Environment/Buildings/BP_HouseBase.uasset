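; House building Blueprint that periodically spawns AI villager mobs at its spawner point until it dies.
; After a random startup delay, a gated retriggerable-delay loop spawns when the game mode's IsVillagerCountAboveMax returns true, then registers the NPC with the game mode.
; Spawns always use the first VillagerMobs entry with the villager behavior tree, though helper functions can add unique classes.
; Death closes the gate shortly afterward, ending the loop.
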(event Custom|Spawning%20Villager
  (bind _villagermobspawner (Variables|Default|GetVillagerMobSpawner))
  (bind _maxdelayspawn (Variables|Default|GetMaxDelaySpawn))
  (bind _returnvalue (Transformation|GetWorldTransform _villagermobspawner))
  ;[1 0 0 1 32] Spawning Villager Mob
  (Utilities|FlowControl|Sequence
    (:then_0
      (goto _label Open))
    (:then_1
      (Utilities|FlowControl|Gate true :!label _label
        (:Exit
          (bind _asbp_third_person_game_mode (Utilities|Casting|CastToBP_ThirdPersonGameMode (Game|GetGameMode)))
          (if (Default|IsVillagerCountAboveMax? _asbp_third_person_game_mode)
            (Utilities|FlowControl|Sequence
              (:then_0
                (bind _returnvalue_2 (AI|SpawnAIFromClass (Utilities|Array|Get(acopy) (Variables|Default|GetVillagerMobs)) "/Game/CourseFiles/Blueprints/AI/VIllager/BT_MobVillager.BT_MobVillager" (.location _returnvalue) (.rotation _returnvalue) false 0))
                (bind _asbp_third_person_game_mode_2 (Utilities|Casting|CastToBP_ThirdPersonGameMode (Game|GetGameMode)))
                (Default|AddNPCtoList _asbp_third_person_game_mode_2 _returnvalue_2))
              (:then_1
                (Utilities|FlowControl|RetriggerableDelay (Math|Random|RandomFloatinRange (/ _maxdelayspawn 0.25) _maxdelayspawn) :!label _label_2)
                (goto _label)))
            (else
              (goto _label_2))))))))

(event Custom|Close%20Loop
  (bind _villagermobspawner (Variables|Default|GetVillagerMobSpawner))
  (bind _maxdelayspawn (Variables|Default|GetMaxDelaySpawn))
  (bind _returnvalue (Transformation|GetWorldTransform _villagermobspawner))
  ;[1 0 0 1 32] Spawning Villager Mob
  (Utilities|FlowControl|Gate true) ; enters at Close
)

(event EventBeginPlay
  (|CallParentFunction)
  (Utilities|FlowControl|Delay (Math|Random|RandomFloatinRange 7.0 9.0))
  (CallFunction|SpawningVillager))

(event Collision|EventActorBeginOverlap
  (params (OtherActor :type Actor%20Object%20Reference))
  (|CallParentFunction OtherActor) ; This node is disabled and will not be called.\nDrag off pins to build functionality.
)

(event EventTick
  (params (DeltaSeconds :type Float%20%28single-precision%29))
  (|CallParentFunction DeltaSeconds) ; This node is disabled and will not be called.\nDrag off pins to build functionality.
)

(event EventPerformDeath
  ;[1 0 0 1 32] Death
  (|CallParentFunction)
  (Utilities|FlowControl|Delay 0.2)
  (CallFunction|CloseLoop))

(fn ConstructionScript
  (|CallParentFunction))

(fn AddVillagerMob
  (params (NewItem :type BP%20Villager%20Base%20Class%20Reference%20%28by%20ref%29))
  (Utilities|Array|AddUnique (Variables|Default|GetVillagerMobs) NewItem))

(fn AddVillagerMobArray
  (params (VillagerMobs1 :type Array%20of%20BP%20Villager%20Base%20Class%20References))
  (for _array_element VillagerMobs1
    (CallFunction|AddVillagerMob _array_element)))