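; Standard house building Blueprint that runs a repeating villager-spawn timer, currently only printing a debug "Spawn Villager" message as a placeholder.
; After a randomized delay on BeginPlay, it opens a Gate and enters it.
; Each pass prints, waits on a randomized retriggerable delay, then re-enters the Gate to form the loop.
; PerformDeath calls the parent, then closes the Gate after a short delay to stop the loop.
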(event Custom|Spawning%20Villager
  ;[1 0 0 1 32] Spawning Villager Mob
  (Utilities|FlowControl|Sequence
    (:then_0
      (goto _label Open))
    (:then_1
      (Utilities|FlowControl|Gate true :!label _label
        (:Exit
          (Utilities|FlowControl|Sequence
            (:then_0
              (Development|PrintString "Spawn Villager"))
            (:then_1
              (Utilities|FlowControl|RetriggerableDelay (Math|Random|RandomFloatinRange 5.0 7.0))
              (goto _label))))))))

(event Custom|Close%20Loop
  ;[1 0 0 1 32] Spawning Villager Mob
  (Utilities|FlowControl|Gate true) ; enters at Close
)

(event EventBeginPlay
  (|CallParentFunction)
  (Utilities|FlowControl|Delay (Math|Random|RandomFloatinRange 7.0 9.0))
  (CallFunction|SpawningVillager))

(event Collision|EventActorBeginOverlap
  (params (OtherActor :type Actor%20Object%20Reference))
  (|CallParentFunction OtherActor) ; This node is disabled and will not be called.\nDrag off pins to build functionality.
)

(event EventTick
  (params (DeltaSeconds :type Float%20%28single-precision%29))
  (|CallParentFunction DeltaSeconds) ; This node is disabled and will not be called.\nDrag off pins to build functionality.
)

(event EventPerformDeath
  ;[1 0 0 1 32] Death
  (|CallParentFunction)
  (Utilities|FlowControl|Delay 0.2)
  (CallFunction|CloseLoop))

(fn ConstructionScript
  (|CallParentFunction))