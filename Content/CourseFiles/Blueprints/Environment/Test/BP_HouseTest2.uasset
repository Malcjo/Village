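; A test destructible house actor that adds itself to the game mode's building count on BeginPlay.
; Point and radial damage of the attack damage type feed BuildingStatsComponent, whose depleted stat sets StateManagerComponent to the Dead state.
; State begin triggers a one-time death that, after a short delay, decrements the count and destroys the actor.
; Combat interface functions for movement and actions return stub values.
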(event OnCurrentStatValueUpdated(BuildingStatsComponent)
  (params (StatType :type E_Stats%20Enum :default "NewEnumerator0") (Value :type Float%20%28double-precision%29))
  (if (and (Utilities|Enum|Equal(Enum) StatType "NewEnumerator1") (<= Value 0.0))
    (Default|SetState (Variables|Default|GetStateManagerComponent) "(TagName=\"Building.State.Dead\")")))

(event OnStateBegin(StateManagerComponent)
  (params (CharacterState :type Gameplay%20Tag%20Structure))
  (|SwitchGameplayTag CharacterState
    (:Building.State.Dead
      (CallFunction|PerformDeath))))

(event Custom|PerformDeath
  ;[1 0 0 1 32] Death
  (if (not (Variables|Default|GetbIsDead?))
    (CallFunction|SetIsDead true)
    (Utilities|FlowControl|Delay 0.2)
    (bind _asbp_third_person_game_mode (Utilities|Casting|CastToBP_ThirdPersonGameMode (Game|GetGameMode)))
    (Variables|/Game/CourseFiles/Blueprints/BP_ThirdPersonGameMode.BP_ThirdPersonGameMode_C|SetNoOfBuidlings _asbp_third_person_game_mode (- (Variables|/Game/CourseFiles/Blueprints/BP_ThirdPersonGameMode.BP_ThirdPersonGameMode_C|GetNoOfBuidlings _asbp_third_person_game_mode) 1))
    (Actor|DestroyActor)))

(event Custom|RecieveDamage
  (params (DamageAmount :type Float%20%28double-precision%29) (DamageType :type Damage%20Type%20Object%20Reference) (InstigatedBy :type Controller%20Object%20Reference) (HitResult :type Hit%20Result%20Structure))
  ;[1 0 0 1 32] Damage
  (bind _asbp_attack_damage_type (Utilities|Casting|CastToBP_AttackDamageType DamageType))
  (Default|TakeDamage (Variables|Default|GetBuildingStatsComponent) DamageAmount)
  (Variables|Default|SetLast%20Hit%20Info HitResult)
  (if (not (Default|IsCurrentStateEqualtoAny? (Variables|Default|GetStateManagerComponent) "(GameplayTags=((TagName=\"Building.State.Dead\")))"))
    _))

(event EventBeginPlay
  (Default|InitialiseStats (Variables|Default|GetBuildingStatsComponent))
  (bind _asbp_third_person_game_mode (Utilities|Casting|CastToBP_ThirdPersonGameMode (Game|GetGameMode)))
  (bind _output_get (Variables|/Game/CourseFiles/Blueprints/BP_ThirdPersonGameMode.BP_ThirdPersonGameMode_C|SetNoOfBuidlings _asbp_third_person_game_mode (+ (Variables|/Game/CourseFiles/Blueprints/BP_ThirdPersonGameMode.BP_ThirdPersonGameMode_C|GetNoOfBuidlings _asbp_third_person_game_mode) 1)))
  (Development|PrintString (Utilities|String|Append "NoOfBuldings: " (Utilities|String|ToString(Integer) _output_get))))

(event Collision|EventActorBeginOverlap
  (params (OtherActor :type Actor%20Object%20Reference)))

(event Game|Damage|EventRadialDamage
  (params (DamageReceived :type Float%20%28single-precision%29) (DamageType :type Damage%20Type%20Object%20Reference) (Origin :type Vector :default "0, 0, 0") (HitInfo :type Hit%20Result%20Structure%20%28by%20ref%29) (InstigatedBy :type Controller%20Object%20Reference) (DamageCauser :type Actor%20Object%20Reference))
  ;[1 0 0 1 32] Damage
  (Development|PrintString (Utilities|GetDisplayName InstigatedBy))
  (CallFunction|RecieveDamage DamageReceived DamageType InstigatedBy HitInfo))

(event EventTick
  (params (DeltaSeconds :type Float%20%28single-precision%29)))

(event Game|Damage|EventPointDamage
  (params (Damage :type Float%20%28single-precision%29) (DamageType :type Damage%20Type%20Object%20Reference) (HitLocation :type Vector :default "0, 0, 0") (HitNormal :type Vector :default "0, 0, 0") (HitComponent :type Primitive%20Component%20Object%20Reference) (BoneName :type Name :default "None") (ShotFromDirection :type Vector :default "0, 0, 0") (InstigatedBy :type Controller%20Object%20Reference) (DamageCauser :type Actor%20Object%20Reference) (HitInfo :type Hit%20Result%20Structure%20%28by%20ref%29))
  ;[1 0 0 1 32] Damage
  (CallFunction|RecieveDamage Damage DamageType InstigatedBy HitInfo))

(fn ConstructionScript)

(fn SetIsDead
  (params (Condition :type Boolean))
  (if (!= Condition (Variables|Default|GetbIsDead?))
    (Variables|Default|SetbIsDead? Condition)))

(fn IsDead
  (return (Variables|Default|GetbIsDead?)))

(fn CanRecieveDamage
  (return (not (Default|IsCurrentStateEqualtoAny? (Variables|Default|GetStateManagerComponent) "(GameplayTags=((TagName=\"Building.State.Dead\")))"))))

(fn GetDesiredRotation
  (return "0, 0, 0"))

(fn GetMovementSpeedMode
  (return "NewEnumerator0"))

(fn GetOwnedGameplayTags
  (return (Variables|Default|GetOwnedGameplayTag)))

(fn HasMatchingGameplayTag
  (params (TagToCheck :type Gameplay%20Tag%20Structure))
  (return (GameplayTags|HasTag (Variables|Default|GetOwnedGameplayTag) TagToCheck)))

(fn PerformAction
  (params (ActionTag :type Gameplay%20Tag%20Structure) (StateTag :type Gameplay%20Tag%20Structure) (MontageIndex :type Integer) (bRandomIndex :type Boolean))
  (return 0.0 false))

(fn PerformAttack
  (params (AttackType :type Gameplay%20Tag%20Structure) (AttackIndex :type Integer) (bRandomIndex? :type Boolean))
  (return 0.0 false))

(fn PerformCustomAction
  (params (ActionTag :type Gameplay%20Tag%20Structure) (StateTag :type Gameplay%20Tag%20Structure) (InMontage :type Anim%20Montage%20Object%20Reference) (MontagePlayRate :type Float%20%28double-precision%29) (bAutoReset? :type Boolean))
  (return false))