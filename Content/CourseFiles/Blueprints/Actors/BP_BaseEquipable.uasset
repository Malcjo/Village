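; Base actor for equipable items held by a character, with an empty PerformItemAction event as a hook for item behavior.
; OnEquipped sets the equipped flag and snaps the item to a named socket on the owning Character's mesh, while OnUnequipped only clears the flag.
; GetItemMesh returns the static mesh component if it has a mesh, otherwise the skeletal one.
; Gameplay tag getters expose the item's tags and support non-exact matching.
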(event Custom|PerformItemAction)

(event EventBeginPlay)

(event Collision|EventActorBeginOverlap
  (params (OtherActor :type Actor%20Object%20Reference)))

(event EventTick
  (params (DeltaSeconds :type Float%20%28single-precision%29)))

(fn ConstructionScript)

(fn GetItemMesh
  (Utilities|IsValid (Variables|/Script/Engine.StaticMeshComponent|GetStaticMesh (Variables|Default|GetItemsStaticMesh))
    (:Is%20Valid
      (return (Variables|Default|GetItemsStaticMesh)))
    (:Is%20Not%20Valid
      (return (Variables|Default|GetItemsSkeletalMesh)))))

(fn OnEquipped
  (CallFunction|SetIsEquipped true)
  (ItemMesh|AttachActor (Variables|Initialization|GetAttachSocket%20Name)))

(fn OnUnequipped
  (if (Variables|Default|GetbIsEquipped?)
    (Variables|Default|SetbIsEquipped? false)))

(fn AttachActor
  (params (SocketName :type Name))
  (Transformation|AttachComponentToComponent (Variables|/Script/Engine.Character|GetMesh (.AsCharacter (Utilities|Casting|CastToCharacter (Components|GetOwner)))) SocketName "SnapToTarget" "SnapToTarget" "SnapToTarget" true))

(fn SetIsEquipped
  (params (IsEquipped :type Boolean))
  (Variables|Default|SetbIsEquipped? IsEquipped))

(fn IsEquipped
  (return (Variables|Default|GetbIsEquipped?)))

(fn GetOwnedGameplayTags
  (return (Variables|GameplayTags|GetOwnedGameplayTags)))

(fn HasMatchingGameplayTag
  (params (TagToCheck :type Gameplay%20Tag%20Structure))
  (return (GameplayTags|HasTag (Variables|GameplayTags|GetOwnedGameplayTags) TagToCheck)))