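; Base equippable weapon actor for melee combat, attached to its owner's hand or stowed socket as combat toggles.
; On equip it registers with the owner's combat component, sends its combat type to the AnimInstance and sets up its collision component.
; Collision hits deal point damage to eligible actors.
; Gameplay tags select action montages, while the owner's current action determines stat cost and damage multiplier.
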(event OnHit(MainWeaponCollisionComponent)
  (params (HitResult :type Hit%20Result%20Structure))
  (bind _hitactor (Collision|BreakHitResult HitResult))
  (bind _returnvalue (Class|BPICombat|CanRecieveDamage(Message) _hitactor))
  (if _returnvalue
    (Game|Damage|ApplyPointDamage _hitactor (Stats|GetDamage) (Transformation|GetActorForwardVector (Components|GetOwner)) HitResult (Game|GetInstigatorController) self (Variables|Initialization|GetDamage%20Type%20Class))))

(event Custom|SimulateWeaponPhysics
  (bind _returnvalue (CallFunction|GetItemMesh))
  (Collision|SetCollisionProfileName _returnvalue "PhysicsActor" true :!class /Script/Engine.PrimitiveComponent)
  (Physics|SetSimulatePhysics _returnvalue false))

(event Custom|ToggleWeaponCombat
  (params (bEnableCombat :type Boolean))
  (CallFunction|AttachActor (select bEnableCombat (Variables|Initialization|GetMainHandSocketName) (Variables|Default|GetAttachSocket%20Name))))

(event EventBeginPlay
  (|CallParentFunction) ; This node is disabled and will not be called.\nDrag off pins to build functionality.
)

(event Collision|EventActorBeginOverlap
  (params (OtherActor :type Actor%20Object%20Reference))
  (|CallParentFunction OtherActor) ; This node is disabled and will not be called.\nDrag off pins to build functionality.
)

(event EventTick
  (params (DeltaSeconds :type Float%20%28single-precision%29))
  (|CallParentFunction DeltaSeconds) ; This node is disabled and will not be called.\nDrag off pins to build functionality.
)

(fn ConstructionScript
  (|CallParentFunction))

(fn OnEquipped
  (|CallParentFunction)
  (bind _output_get (Variables|Default|SetCombatComponent (Actor|GetComponentbyClass (Components|GetOwner) "/Game/CourseFiles/Blueprints/Components/BP_CombatComponent.BP_CombatComponent_C")))
  (EventDispatchers|BindEventtoOnCombatToggled (Variables|Default|GetCombatComponent) (EventDispatchers|CreateEvent :!event Custom|ToggleWeaponCombat))
  (Variables|Default|SetOwnerStateManager (Actor|GetComponentbyClass (Components|GetOwner) "/Game/CourseFiles/Blueprints/Components/BP_StateManagerComponent.BP_StateManagerComponent_C"))
  ;[1 1 1] Needs to have a set stat component here from video but he never made it, leaving here just in case he does in future otherwise I'll have to figure it out, if breaks check here
  (Variables|Default|SetOwnerStatsComponent (Actor|GetComponentbyClass (Components|GetOwner) "/Game/CourseFiles/Blueprints/Components/BP_StatsComponent.BP_StatsComponent_C"))
  (CallFunction|AttachActor (select (Default|IsCombatEnabled? (Variables|Default|GetCombatComponent)) (Variables|Initialization|GetMainHandSocketName) (Variables|Default|GetAttachSocket%20Name)))
  (Default|SetMainWeapon (Variables|Default|GetCombatComponent) self)
  (Class|BPIAnimInstance|UpdateCombatType(Message) (Components|SkeletalMesh|GetAnimInstance (Variables|/Script/Engine.Character|GetMesh (.AsCharacter (Utilities|Casting|CastToCharacter (Components|GetOwner))))) (Variables|Initialization|GetCombatType))
  (Default|SetCollisionMesh (Variables|Default|GetMainWeaponCollisionComponent) (CallFunction|GetItemMesh))
  (Default|AddActortoIgnore (Variables|Default|GetMainWeaponCollisionComponent) (Components|GetOwner)))

(fn GetActionMontages
  (params (CharacterAction :type Gameplay%20Tag%20Structure))
  (|SwitchGameplayTag CharacterAction
    (:Character.Action.Attack.Light%20Attack
      (return (Variables|Montages|GetLightAttackMontages)))
    (:Character.Action.Attack.Heavy%20Attack
      (return (Variables|Montages|GetHeavyAttackMontages)))
    (:Character.Action.Attack.Charged%20Attack
      (return (Variables|Montages|GetChargedAttackMontages)))
    (:Character.Action.Attack.Sprint%20Attack
      (return (Variables|Montages|GetSprintAttackMontages)))
    (:Character.Action.Attack.Falling%20Attack
      (return (Variables|Montages|GetFallingAttackMontages)))
    (:Character.Action.Dodge
      (return (Variables|Montages|GetDodgeMontages)))
    (:Character.Action.Enter%20Combat
      (return (Utilities|Array|MakeArray (Variables|Montages|GetEnterCombat))))
    (:Character.Action.Exit%20Combat
      (return (Utilities|Array|MakeArray (Variables|Montages|GetExitCombat))))
    (:Character.Action.Block
      (return (Variables|Montages|GetBlockMontages)))))

(fn GetStatCostforAction
  (bind _ownerstatemanager (Variables|Default|GetOwnerStateManager)
    (:then
      (return (.Value (Utilities|Map|Find (Variables|Stats|GetActionStatCost) (Default|GetCurrentCharacterAction _ownerstatemanager)))))
    (:else
      (return 0.0))))

(fn GetDamage
  (bind _damage (Variables|Stats|GetDamage))
  (bind _ownerstatemanager (Variables|Default|GetOwnerStateManager)
    (:then
      (return (* _damage (Math|Float|Clamp(Float) (.Value (Utilities|Map|Find (Variables|Stats|GetActionDamageMultiplier) (Default|GetCurrentCharacterAction _ownerstatemanager))) 1.0 (.Value (Utilities|Map|Find (Variables|Stats|GetActionDamageMultiplier) (Default|GetCurrentCharacterAction _ownerstatemanager)))))))
    (:else
      (return _damage))))

(fn ActivateCollision
  (params (CollisionPart :type E_CollisionPart%20Enum :default "NewEnumerator0"))
  (Default|ActivateCollision (Variables|Default|GetMainWeaponCollisionComponent)))

(fn DeactivateCollision
  (params (CollisionPart :type E_CollisionPart%20Enum :default "NewEnumerator0"))
  (Default|DeactivateCollision (Variables|Default|GetMainWeaponCollisionComponent)))