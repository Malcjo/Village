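; Boss enemy character that fights with a melee weapon and shows its own on-screen health bar while it has a target.
; BeginPlay initialises stats, weapon collision and the health widget.
; Weapon collision hits apply stat-based point damage to actors that accept it.
; Combat toggles move the weapon between sockets, and death hides the bar and changes the weapon's collision profile, with physics simulation left off.
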(event OnHit(SecondaryWeaponCollisionComponent)
  (params (HitResult :type Hit%20Result%20Structure))
  ;[1 0 0 1 32] Damage
  (CallFunction|HitEvent HitResult))

(event OnHit(MainWeaponCollisionComponent)
  (params (HitResult :type Hit%20Result%20Structure))
  ;[1 0 0 1 32] Damage
  (CallFunction|HitEvent HitResult))

(event OnCombatToggled(CombatComponent)
  (params (bIsCombatEnabled? :type Boolean))
  ;[1 0 0 1 32] Toggle Combat
  (Transformation|AttachComponentToComponent (Variables|Default|GetWeaponMesh) (Variables|Character|GetMesh) (select bIsCombatEnabled? (Variables|Initialization|GetWeapon%20Hand%20Socket%20Name) (Variables|Initialization|GetAttach%20Socket%20Name)) "SnapToTarget" "SnapToTarget" "SnapToTarget" true))

(event Custom|SimulateWeaponPhysics
  (bind _weaponmesh (Variables|Default|GetWeaponMesh))
  (Collision|SetCollisionProfileName _weaponmesh "PhysicsActor" true :!class /Script/Engine.PrimitiveComponent)
  (Physics|SetSimulatePhysics _weaponmesh false))

(event Custom|SetBossHealthVisibility
  (params (bVisible? :type Boolean))
  ;[1 0 0 1 32] Visualize HealthBar
  (bind _bosshealthui (Variables|Default|GetBossHealthUI)
    (:then
      (Widget|SetVisibility _bosshealthui (select (and bVisible? (not (Default|IsCurrentStateEqualtoAny? (Variables|Default|GetStateManagerComponent) "(GameplayTags=((TagName=\"Character.State.Dead\")))"))) "Visible" "Hidden")))
    (:else)))

(event Custom|Hit%20Event
  (params (Hit :type Hit%20Result%20Structure%20%28by%20ref%29))
  (bind _hitactor (Collision|BreakHitResult Hit))
  ;[1 0 0 1 32] Damage
  (Utilities|IsValid _hitactor
    (:Is%20Valid
      (bind _returnvalue (Class|BPICombat|CanRecieveDamage(Message) _hitactor))
      (if _returnvalue
        (Game|Damage|ApplyPointDamage _hitactor (Default|GetCurrentStatValue (Variables|Default|GetStatsComponent) "NewEnumerator4") (Transformation|GetActorForwardVector) Hit (Pawn|GetController) self "/Game/CourseFiles/Blueprints/DamageTypes/BP_AttackDamageType.BP_AttackDamageType_C")))))

(event EventBeginPlay
  ;[1 0 0 1 32] Intitalize
  (|CallParentFunction)
  (CallFunction|SetCanTakeDamagebyPlayer true)
  (Default|InitialiseStats (Variables|Default|GetStatsComponent))
  (Default|SetCollisionMesh (Variables|Default|GetMainWeaponCollisionComponent) (Variables|Default|GetWeaponMesh))
  (bind _returnvalue (UserInterface|CreateWidget "/Game/CourseFiles/UI/WB_BossHealth.WB_BossHealth_C" (Game|GetPlayerController 0)))
  (bind _output_get (Variables|Default|SetBossHealthUI _returnvalue))
  (Default|Initalize _output_get (Variables|Default|GetStatsComponent))
  (UserInterface|Viewport|AddtoViewport (Variables|Default|GetBossHealthUI) 0))

(event Collision|EventActorBeginOverlap
  (params (OtherActor :type Actor%20Object%20Reference)))

(event EventTick
  (params (DeltaSeconds :type Float%20%28single-precision%29)))

(event EventOnTargeted
  (params (bIsTargetted :type Boolean))
  ;[1 0 0 1 32] Targetted
  (|CallParentFunction bIsTargetted))

(event EventPerformDeath
  ;[1 0 0 1 32] Death
  (|CallParentFunction)
  (CallFunction|SimulateWeaponPhysics)
  (CallFunction|SetBossHealthVisibility false))

(event EventOnTargetSet
  (params (NewTarget :type Actor%20Object%20Reference))
  ;[1 0 0 1 32] Targetted
  (|CallParentFunction NewTarget)
  (CallFunction|SetBossHealthVisibility (Utilities|IsValid NewTarget)))

(fn ConstructionScript
  (|CallParentFunction))