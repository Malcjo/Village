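; BP_Boss_Troll is the troll boss character Blueprint, extending a parent class.
; On BeginPlay it runs the parent logic, then points its main and secondary weapon collision components at the character mesh.
; HasMatchingGameplayTag always returns false, and the construction script only calls the parent.
; An unconnected spawn-climb montage call never runs, and the Tick and overlap events are disabled.
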(event EventBeginPlay
  (|CallParentFunction)
  (Default|SetCollisionMesh (Variables|Default|GetMainWeaponCollisionComponent) (Variables|Character|GetMesh))
  (Default|SetCollisionMesh (Variables|Default|GetSecondaryWeaponCollisionComponent) (Variables|Character|GetMesh)))

(event Collision|EventActorBeginOverlap
  (params (OtherActor :type Actor%20Object%20Reference))
  (|CallParentFunction OtherActor) ; This node is disabled and will not be called.\nDrag off pins to build functionality.
)

(event EventTick
  (params (DeltaSeconds :type Float%20%28single-precision%29))
  (|CallParentFunction DeltaSeconds) ; This node is disabled and will not be called.\nDrag off pins to build functionality.
)

(fn ConstructionScript
  (|CallParentFunction))

(fn HasMatchingGameplayTag
  (params (TagToCheck :type Gameplay%20Tag%20Structure))
  (return false))