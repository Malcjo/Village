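; AI controller for a boss that senses and targets houses and the player.
; On possess it runs the BP_MasterAI pawn's behavior tree and mirrors combat toggles into the Blackboard.
; Perception updates filter successful stimuli by index and gameplay tag: the first accepts houses or players, the second only players.
; Matches set the Blackboard Target and notify the pawn; live logic never clears it, and GetValidActors is unused.
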(event OnPerceptionUpdated(AIPerception)
  (params (UpdatedActors :type Array%20of%20Actor%20Object%20References))
  (CallFunction|UpdatePerception UpdatedActors))

(event Custom|OnCombatToggled
  (params (bIsCombatEnabled? :type Boolean))
  (AI|Components|Blackboard|SetValueasBool (Variables|Default|GetBlackboard) (Utilities|Name|MakeLiteralName "bCombatEnabled") bIsCombatEnabled?))

(event EventBeginPlay)

(event EventTick
  (params (DeltaSeconds :type Float%20%28single-precision%29)))

(event EventPossess
  (params (PossessedPawn :type Pawn%20Object%20Reference))
  (bind _asbp_master_ai (Utilities|Casting|CastToBP_MasterAI PossessedPawn))
  (Variables|Default|SetMaster%20AI _asbp_master_ai)
  (EventDispatchers|BindEventtoOnCombatToggled (Variables|/Game/CourseFiles/Blueprints/AI/BP_MasterAI.BP_MasterAI_C|GetCombatComponent (Variables|Default|GetMaster%20AI)) (delegate Custom|OnCombatToggled))
  (AI|RunBehaviorTree (Variables|/Game/CourseFiles/Blueprints/AI/BP_MasterAI.BP_MasterAI_C|GetBehavior%20Tree (Variables|Default|GetMaster%20AI))))

(fn ConstructionScript)

(fn UpdatePerception
  (params (PercievedActors :type Array%20of%20Actor%20Object%20References))
  (for _array_element PercievedActors
    (LocalVariables|SetL_SensedActor _array_element)
    (bind _info (Class|AIPerceptionComponent|GetActorsPerception (Variables|Default|GetAIPerception) (LocalVariables|GetL_SensedActor)))
    (for (_array_element_2 _array_index) (.LastSensedStimuli (Utilities|Struct|BreakActorPerceptionBlueprintInfo _info))
      (LocalVariables|SetL_AIStimilus _array_element_2)
      (switch int _array_index
        (:0
          (Development|PrintString "Sense House" true true "(R=0.000000,G=0.660000,B=1.000000,A=1.000000)" 1e+01)
          (if (.bSuccessfullySensed (Utilities|Struct|BreakAIStimulus (LocalVariables|GetL_AIStimilus)))
            (bind _returnvalue (Class|GameplayTagBlueprintInterface|HasMatchingGameplayTag(Message) (LocalVariables|GetL_SensedActor) "(TagName=\"Building.Standard.House\")"))
            (if _returnvalue
              (CallFunction|SetTargetActor (LocalVariables|GetL_SensedActor))
              (else
                (Development|PrintString "Sense Player" true true "(R=0.000000,G=0.660000,B=1.000000,A=1.000000)" 1e+01 :!label _label)
                (if (.bSuccessfullySensed (Utilities|Struct|BreakAIStimulus (LocalVariables|GetL_AIStimilus)))
                  (bind _returnvalue_2 (Class|GameplayTagBlueprintInterface|HasMatchingGameplayTag(Message) (LocalVariables|GetL_SensedActor) "(TagName=\"Character.Player\")"))
                  (if _returnvalue_2
                    (CallFunction|SetTargetActor (LocalVariables|GetL_SensedActor))))))))
        (:1
          (goto _label))))))

(fn SetTargetActor
  (params (NewTargetActor :type Actor%20Object%20Reference))
  (AI|Components|Blackboard|SetValueasObject (Variables|Default|GetBlackboard) (Utilities|Name|MakeLiteralName "Target") NewTargetActor)
  (bind _master_ai (Variables|Default|GetMaster%20AI)
    (:then
      (Default|OnTargetSet _master_ai NewTargetActor))
    (:else)))

(fn GetValidActors
  (params (Valid%20Actors :type Array%20of%20Actor%20Object%20References))
  (for _array_element Valid%20Actors
    (LocalVariables|SetL_SensedActor _array_element)
    (bind _info (Class|AIPerceptionComponent|GetActorsPerception (Variables|Default|GetAIPerception) (LocalVariables|GetL_SensedActor)))
    (for (_array_element_2 _array_index) (.LastSensedStimuli (Utilities|Struct|BreakActorPerceptionBlueprintInfo _info))
      (LocalVariables|SetL_AIStimilus _array_element_2)
      (switch int _array_index
        (:0
          (if (.bSuccessfullySensed (Utilities|Struct|BreakAIStimulus (LocalVariables|GetL_AIStimilus)))
            (bind _returnvalue (Class|GameplayTagBlueprintInterface|HasMatchingGameplayTag(Message) (LocalVariables|GetL_SensedActor) "(TagName=\"Building.Standard.House\")"))
            (if _returnvalue
              (Utilities|Array|AddUnique Valid%20Actors (LocalVariables|GetL_SensedActor))
              (else
                (bind _returnvalue_2 (Class|GameplayTagBlueprintInterface|HasMatchingGameplayTag(Message) (LocalVariables|GetL_SensedActor) "(TagName=\"Building.Standard.House\")"))
                (if _returnvalue_2
                  (Utilities|Array|AddUnique Valid%20Actors (LocalVariables|GetL_SensedActor)))))))
        (:1
          (if (.bSuccessfullySensed (Utilities|Struct|BreakAIStimulus (LocalVariables|GetL_AIStimilus)))
            (bind _returnvalue_3 (Class|GameplayTagBlueprintInterface|HasMatchingGameplayTag(Message) (LocalVariables|GetL_SensedActor) "(TagName=\"Building.Standard.House\")"))
            (if _returnvalue_3
              (CallFunction|SetTargetActor (LocalVariables|GetL_SensedActor)))))))))