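; Base villager AI character with stats, a melee weapon and a targeting health bar, set up not to take damage from the player.
; Weapon collision hits apply point damage from StatsComponent to actors that can receive it, while the villager's own CanRecieveDamage returns false.
; Combat toggles snap the weapon between hand and attach sockets.
; Death switches the weapon to the PhysicsActor collision profile but leaves physics simulation off.
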(event OnHit(MainWeaponCollisionComponent)
  (params (HitResult :type Hit%20Result%20Structure))
  (bind _hitactor (Collision|BreakHitResult HitResult))
  (bind _returnvalue (Class|BPICombat|CanRecieveDamage(Message) _hitactor))
  (if _returnvalue
    (Game|Damage|ApplyPointDamage _hitactor (Default|GetCurrentStatValue (Variables|Default|GetStatsComponent) "NewEnumerator4") (Transformation|GetActorForwardVector) HitResult (Pawn|GetController) self "/Game/CourseFiles/Blueprints/DamageTypes/BP_AttackDamageType.BP_AttackDamageType_C")))

(event OnCombatToggled(CombatComponent)
  (params (bIsCombatEnabled? :type Boolean))
  (Transformation|AttachComponentToComponent (CallFunction|GetWeaponMesh) (Variables|Character|GetMesh) (select bIsCombatEnabled? (Variables|Initialization|GetWeapon%20Hand%20Socket%20Name) (Variables|Initialization|GetAttach%20Socket%20Name)) "SnapToTarget" "SnapToTarget" "SnapToTarget" true))

(event Custom|SimulateWeaponPhysics
  (bind _returnvalue (CallFunction|GetWeaponMesh))
  (Collision|SetCollisionProfileName _returnvalue "PhysicsActor" true :!class /Script/Engine.PrimitiveComponent)
  (Physics|SetSimulatePhysics _returnvalue false))

(event EventBeginPlay
  (|CallParentFunction)
  (CallFunction|SetCanTakeDamagebyPlayer false)
  (Default|InitialiseStats (Variables|Default|GetStatsComponent))
  (Default|SetCollisionMesh (Variables|Default|GetMainWeaponCollisionComponent) (CallFunction|GetWeaponMesh))
  (bind _returnvalue (UserInterface|CreateWidget "/Game/CourseFiles/UI/WB_HealthBar.WB_HealthBar_C" (Game|GetPlayerController 0) (Variables|Default|GetStatsComponent)))
  (UserInterface|SetWidget (Variables|Default|GetHealthBarWidget) _returnvalue))

(event Collision|EventActorBeginOverlap
  (params (OtherActor :type Actor%20Object%20Reference)))

(event EventTick
  (params (DeltaSeconds :type Float%20%28single-precision%29)))

(event EventOnTargeted
  (params (bIsTargetted :type Boolean))
  (|CallParentFunction bIsTargetted)
  (Rendering|SetVisibility (Variables|Default|GetHealthBarWidget) bIsTargetted false))

(event EventPerformDeath
  (|CallParentFunction)
  (CallFunction|SimulateWeaponPhysics))

(fn ConstructionScript
  (|CallParentFunction))

(fn CanRecieveDamage
  (return false))