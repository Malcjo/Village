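; Boss AI controller (named OLD) that picks targets from AI perception, favoring no priority between houses and players.
; On perception updates, UpdatePerception treats stimulus index as the sense: index 0 targets House-tagged actors, index 1 Player-tagged ones, via SetTargetActor.
; Behavior tree startup and combat-toggle binding to the bCombatEnabled blackboard key are disconnected.
; SetSight and GetValidActors are alternative targeting helpers with no live caller here.
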(event OnPerceptionUpdated(AIPerception)
  (params (UpdatedActors :type Array%20of%20Actor%20Object%20References))
  (Development|PrintString "Update Boss AIPerception")
  (CallFunction|UpdatePerception UpdatedActors))

(event Custom|CustomEvent
  (params (bIsCombatEnabled? :type Boolean))
  (AI|Components|Blackboard|SetValueasBool (Variables|Default|GetBlackboard) (Utilities|Name|MakeLiteralName "bCombatEnabled") bIsCombatEnabled?))

(event EventBeginPlay
  (|CallParentFunction) ; This node is disabled and will not be called.\nDrag off pins to build functionality.
)

(event EventTick
  (params (DeltaSeconds :type Float%20%28single-precision%29)))

(fn ConstructionScript
  (|CallParentFunction))

(fn UpdatePerception
  (params (PercievedActors :type Array%20of%20Actor%20Object%20References))
  (for _array_element PercievedActors
    (LocalVariables|SetL_SensedActor _array_element)
    (bind _info (Class|AIPerceptionComponent|GetActorsPerception (Variables|Default|GetAIPerception) (LocalVariables|GetL_SensedActor)))
    (for (_array_element_2 _array_index) (.LastSensedStimuli (Utilities|Struct|BreakActorPerceptionBlueprintInfo _info))
      (LocalVariables|SetL_AIStimilus _array_element_2)
      (switch int _array_index
        (:0
          (Development|PrintString "Check Buildings" true true "(R=0.000000,G=0.660000,B=1.000000,A=1.000000)" 1e+01)
          (if (.bSuccessfullySensed (Utilities|Struct|BreakAIStimulus (LocalVariables|GetL_AIStimilus)))
            (bind _returnvalue (Class|GameplayTagBlueprintInterface|HasMatchingGameplayTag(Message) (LocalVariables|GetL_SensedActor) "(TagName=\"Building.Standard.House\")"))
            (if _returnvalue
              (CallFunction|SetTargetActor (LocalVariables|GetL_SensedActor)))))
        (:1
          (Development|PrintString "Check for players, or villagers" true true "(R=0.000000,G=0.660000,B=1.000000,A=1.000000)" 1e+01)
          (if (.bSuccessfullySensed (Utilities|Struct|BreakAIStimulus (LocalVariables|GetL_AIStimilus)))
            (bind _returnvalue_2 (Class|GameplayTagBlueprintInterface|HasMatchingGameplayTag(Message) (LocalVariables|GetL_SensedActor) "(TagName=\"Character.Player\")"))
            (if _returnvalue_2
              (CallFunction|SetTargetActor (LocalVariables|GetL_SensedActor)))))))))

(fn SetSight
  (params (Actor :type Object%20Object%20Reference) (Stimulus :type AI%20Stimulus%20Structure%20%28by%20ref%29))
  (bind (_age _expirationage _strength _stimuluslocation _receiverlocation _tag _bsuccessfullysensed) (Utilities|Struct|BreakAIStimulus Stimulus))
  (bind _returnvalue (Class|AIPerceptionSystem|GetSenseClassforStimulus Stimulus))
  (if (== _returnvalue "/Script/AIModule.AISense_Sight")
    (bind _returnvalue_2 (Class|GameplayTagBlueprintInterface|HasMatchingGameplayTag(Message) Actor "(TagName=\"Building.Standard.House\")"))
    (if _returnvalue_2
      (Development|PrintString "House")
      (AI|Components|Blackboard|SetValueasObject (Variables|Default|GetBlackboard) (Utilities|Name|MakeLiteralName "Target") (Utilities|SelectObject Actor 0 _bsuccessfullysensed))
      (if (not _bsuccessfullysensed)
        (AI|Components|Blackboard|SetValueasVector (Variables|Default|GetBlackboard) (Utilities|Name|MakeLiteralName "TargetLocation") _stimuluslocation))
      (else
        (Development|PrintString "Not House")
        (Development|PrintString (Utilities|GetDisplayName Actor))
        (return)))
    (else
      (Development|PrintString "No Sense")
      (return))))

(fn GetValidActors
  (params (PercievedActors :type Array%20of%20Actor%20Object%20References))
  (for _array_element PercievedActors
    (LocalVariables|SetL_SensedActor _array_element)
    (bind _info (Class|AIPerceptionComponent|GetActorsPerception (Variables|Default|GetAIPerception) (LocalVariables|GetL_SensedActor)))
    (for (_array_element_2 _array_index) (.LastSensedStimuli (Utilities|Struct|BreakActorPerceptionBlueprintInfo _info))
      (LocalVariables|SetL_AIStimilus _array_element_2)
      (switch int _array_index
        (:0
          (if (.bSuccessfullySensed (Utilities|Struct|BreakAIStimulus (LocalVariables|GetL_AIStimilus)))
            (bind _returnvalue (Class|GameplayTagBlueprintInterface|HasMatchingGameplayTag(Message) (LocalVariables|GetL_SensedActor) "(TagName=\"Building.Standard.House\")"))
            (if _returnvalue
              (Utilities|Array|AddUnique (Variables|Default|GetValidActors) (LocalVariables|GetL_SensedActor))
              (else
                (bind _returnvalue_2 (Class|GameplayTagBlueprintInterface|HasMatchingGameplayTag(Message) (LocalVariables|GetL_SensedActor) "(TagName=\"Building.Standard.House\")"))
                (if _returnvalue_2
                  (Utilities|Array|AddUnique (Variables|Default|GetValidActors) (LocalVariables|GetL_SensedActor)))))))
        (:1
          (if (.bSuccessfullySensed (Utilities|Struct|BreakAIStimulus (LocalVariables|GetL_AIStimilus)))
            (bind _returnvalue_3 (Class|GameplayTagBlueprintInterface|HasMatchingGameplayTag(Message) (LocalVariables|GetL_SensedActor) "(TagName=\"Building.Standard.House\")"))
            (if _returnvalue_3
              (CallFunction|SetTargetActor (LocalVariables|GetL_SensedActor)))))))))