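; Dummy character that acts as a lock-on target, with stats and a state manager.
; BeginPlay initialises the stats component, and OnTargeted shows or hides the lock-on widget.
; CanBeTargetted allows targeting unless the state manager reports the Dead state.
; Damage, hit reaction and starting-equipment spawning logic sits in the event graph but is unconnected, so it never runs.
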(event EventBeginPlay
  (Default|InitialiseStats (Variables|Default|GetStatsComponent)))

(event Collision|EventActorBeginOverlap
  (params (OtherActor :type Actor%20Object%20Reference)))

(event EventTick
  (params (DeltaSeconds :type Float%20%28single-precision%29)))

(event EventOnTargeted
  (params (bIsTargetted :type Boolean))
  (Rendering|SetVisibility (Variables|Default|GetLockOnWidget) bIsTargetted false))

(fn ConstructionScript
  (|CallParentFunction))

(fn CanbeTargetted
  (return (not (Default|IsCurrentStateEqualtoAny? (Variables|Default|GetStateManagerComponent) "(GameplayTags=((TagName=\"Character.State.Dead\")))"))))